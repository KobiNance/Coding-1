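; BP_tree is a tree Blueprint that grows in steps when play begins.
; BeginPlay runs a delayed loop while Growcounter is above zero, waiting a short random interval before each step.
; Each step adds a random amount to the static mesh's relative scale and decrements the counter, so growth timing and final size vary.
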(event `self.ReceiveBeginPlay`
  (bind _staticmesh (`self.StaticMesh`))
  (if (> (`self.growcounter`) 0) :!label _label
    (`KismetSystemLibrary.Delay` (`KismetMathLibrary.RandomFloatInRange` 0.4 0.6))
    (`SceneComponent.SetRelativeScale3D` _staticmesh (+ (`SceneComponent.RelativeScale3D` _staticmesh) (`KismetMathLibrary.RandomFloatInRange` 0.2 0.4)))
    (`/Engine/EditorBlueprintResources/StandardMacros.DecrementInt` (`self.growcounter`) ; subtract 1 from growth counter
      (:`  `
        (goto _label)))))

(fn `UserConstructionScript`)