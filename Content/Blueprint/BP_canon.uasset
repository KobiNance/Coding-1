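; BP_canon is a cannon actor that launches an overlapping third-person character along its Cube's forward vector.
; Overlap, or BeginPlay after a delay, calls LaunchCannonball, which prints "Ka-pow".
; Both the caller and that event flow into a cast of the overlap's OtherActor, then enable capsule physics and add the Force.
; A node to spawn BP_cannonball exists but is unconnected.
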(event `self.ReceiveBeginPlay`
  (`KismetSystemLibrary.Delay` 15.0)
  (`self.Launch cannonball` :!label _label)
  (bind _asbp_third_person_character (cast `/Game/ThirdPerson/Blueprints/BP_ThirdPersonCharacter` (stale `self.ReceiveActorBeginOverlap` OtherActor) :!label _label_2))
  (`PrimitiveComponent.SetSimulatePhysics` (`Character.CapsuleComponent` _asbp_third_person_character) true)
  (`PrimitiveComponent.AddForce` (`Character.CapsuleComponent` _asbp_third_person_character) (* (`SceneComponent.GetForwardVector` (`self.cube`)) (`self.force`)) "None" false))

(event `self.ReceiveActorBeginOverlap`
  (params (OtherActor :type "Actor Object Reference"))
  (goto _label))

(event `Launch cannonball`
  (`KismetSystemLibrary.PrintText` "Ka-pow")
  (goto _label_2))

(fn `UserConstructionScript`)