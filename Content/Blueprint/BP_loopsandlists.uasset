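; BP_loopsandlists is an actor Blueprint that demonstrates loops and arrays through printed text and moving keys.
; On BeginPlay, a delayed while loop counts Whilecounter down, printing each number in a color picked from the Colors array by modulo.
; A second delayed branch starts Makecoinsjump, which raises every BP_Key actor, prints the count, then calls itself after a delay, so keys keep rising indefinitely.
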(event `self.ReceiveBeginPlay`
  (bind _whilecounter (`self.whilecounter`))
  (`|ExecutionSequence`
    (:`then_0`
      (`KismetSystemLibrary.Delay` 2.0)
      (while (> _whilecounter 0)
        (`KismetSystemLibrary.PrintText` (`|FormatText` "we are in loop number {count}" _whilecounter) true true (`|GetArrayItem` (`self.colors`) (mod (`self.whilecounter`) 7)) 22.0)
        (`/Engine/EditorBlueprintResources/StandardMacros.DecrementInt` (`self.whilecounter`))))
    (:`then_1`
      (`KismetSystemLibrary.Delay` 1.0)
      (`self.Makecoinsjump`))))

(event `Makecoinsjump`
  (bind _outactors (`GameplayStatics.GetAllActorsOfClass` "/Game/Blueprint/BP_Key.BP_Key_C"))
  (for _array_element _outactors
    (`SceneComponent.K2_AddRelativeLocation` (`/Game/Blueprint/BP_Key.DefaultSceneRoot` _array_element) (0.0 0.0 50.0) false false))
  (`KismetSystemLibrary.PrintText` (`|FormatText` "we have raised {count} keys" (`KismetArrayLibrary.Array_Length` _outactors)) true true (struct :`G` 0.66 :`B` 1.0 :`A` 1.0) 22.0)
  (`KismetSystemLibrary.Delay` 1.0)
  (`self.Makecoinsjump`))

(fn `UserConstructionScript`)