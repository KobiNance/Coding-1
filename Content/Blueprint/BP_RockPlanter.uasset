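; BP_RockPlanter is a pickup item that can be held by the third-person character and used to spawn a tree.
; On overlap it stores the character as Player and passes itself to that character's PickUpItem.
; PlantSeed spawns BP_tree at the planter's transform.
; Event names are swapped relative to behavior: Drop attaches to the player mesh's HandGrip_R socket, while PickUp destroys the actor.
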(event `self.ReceiveActorBeginOverlap`
  (params (OtherActor :type "Actor Object Reference"))
  (bind _asbp_third_person_character (cast `/Game/ThirdPerson/Blueprints/BP_ThirdPersonCharacter` OtherActor))
  (set `self.Player` _asbp_third_person_character)
  (`/Game/ThirdPerson/Blueprints/BP_ThirdPersonCharacter.PickUpItem` _asbp_third_person_character self))

(event `/Game/Blueprint/I_seedplanter.Drop`
  (`KismetSystemLibrary.PrintText` "This rock planter has been picked up")
  (`self.K2_AttachToComponent` (`Character.Mesh` (`self.Player`)) "HandGrip_R" "SnapToTarget" "SnapToTarget" "KeepRelative"))

(event `/Game/Blueprint/I_seedplanter.PlantSeed`
  (`KismetSystemLibrary.PrintText` "Trying to plant rocks")
  (`|SpawnActorFromClass` "/Game/Blueprint/BP_tree.BP_tree_C" (`self.GetTransform`) "Undefined" "MultiplyWithRoot" null null))

(event `/Game/Blueprint/I_seedplanter.PickUp`
  (`KismetSystemLibrary.PrintText` "trying to drop the planter")
  (`self.K2_DestroyActor`))

(fn `UserConstructionScript`)